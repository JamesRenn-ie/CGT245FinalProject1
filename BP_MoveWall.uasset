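; BP_MoveWall is a wall actor that slides from a start point to an end point when its ButtonTouched event fires.
; A timeline lerps the static mesh's world location between the StartWall and EndWall components.
; MovePlatform gates playback through a FlipFlop with only A wired.
; The timeline's Finished re-calls MovePlatform, normally consuming the empty B branch so the next trigger replays from the start.
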(event Custom|MovePlatform
  (Utilities|FlowControl|FlipFlop
    (:A
      (bind _alpha (Timeline|Timeline PlayFromStart)
        (:Update
          (Transformation|SetWorldLocation (Variables|Default|GetStaticMesh) (Math|Vector|Lerp(Vector) (Transformation|GetWorldLocation (Variables|Default|GetStartWall)) (Transformation|GetWorldLocation (Variables|Default|GetEnd%20Wall)) _alpha) false false))
        (:Finished
          (CallFunction|MovePlatform))))))

(event Custom|ButtonTouched
  (CallFunction|MovePlatform))

(event Collision|EventActorBeginOverlap
  (params (OtherActor :type Actor%20Object%20Reference)))

(event EventTick
  (params (DeltaSeconds :type Float%20%28single-precision%29)))

(fn ConstructionScript)