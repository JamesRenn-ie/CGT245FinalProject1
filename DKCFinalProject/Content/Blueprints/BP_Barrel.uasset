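; BP_Barrel is a hazard that chases the third-person player and ends the game on contact.
; BeginPlay caches the player character, and Tick steps the barrel one unit per frame toward the player's XY position at world Z zero, without sweep or delta-time scaling.
; When its Box overlaps the character, it shows the LoseScreen widget, pauses the game and destroys that character.
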(event OnComponentBeginOverlap(Box)
  (params (OverlappedComponent :type Primitive%20Component%20Object%20Reference) (OtherActor :type Actor%20Object%20Reference) (OtherComp :type Primitive%20Component%20Object%20Reference) (OtherBodyIndex :type Integer) (bFromSweep :type Boolean) (SweepResult :type Hit%20Result%20Structure%20%28by%20ref%29))
  (bind _asbp_third_person_character (Utilities|Casting|CastToBP_ThirdPersonCharacter OtherActor))
  (bind _returnvalue (UserInterface|CreateWidget "/Game/Blueprints/LoseScreen.LoseScreen_C"))
  (UserInterface|Viewport|AddtoViewport _returnvalue 0)
  (Game|SetGamePaused true)
  (Actor|DestroyActor _asbp_third_person_character))

(event EventBeginPlay
  (bind _asbp_third_person_character (Utilities|Casting|CastToBP_ThirdPersonCharacter (Game|GetPlayerCharacter 0)))
  (Variables|Default|SetAs%20BP%20Third%20Person%20Character _asbp_third_person_character))

(event Collision|EventActorBeginOverlap
  (params (OtherActor :type Actor%20Object%20Reference)))

(event EventTick
  (params (DeltaSeconds :type Float%20%28single-precision%29))
  (Transformation|SetActorLocation (+ (Transformation|GetActorLocation) (Math|Vector|Normalize (- (* (Transformation|GetActorLocation (Variables|Default|GetAs%20BP%20Third%20Person%20Character)) "1.000000,1.000000,0.000000") (Transformation|GetActorLocation)))) false false))

(fn ConstructionScript)