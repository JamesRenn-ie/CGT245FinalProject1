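; BP_Platform is a moving platform that shuttles its Cube back and forth between the StartPos and EndPos components.
; BeginPlay calls MovePlatform, where a FlipFlop alternates between playing the timeline forward and reversing it from the end.
; Timeline updates lerp the cube's world location without sweep, and the Finished output calls MovePlatform again to keep the motion looping.
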(event Custom|MovePlatform
  (Utilities|FlowControl|FlipFlop
    (:A
      (bind _alpha (Timeline|Timeline PlayFromStart)
        (:Update
          (Transformation|SetWorldLocation (Variables|Default|GetCube) (Math|Vector|Lerp(Vector) (Transformation|GetWorldLocation (Variables|Default|GetstartPos)) (Transformation|GetWorldLocation (Variables|Default|GetendPos)) _alpha) false false))
        (:Finished
          (CallFunction|MovePlatform))))
    (:B
      (Timeline|Timeline ReverseFromEnd))))

(event EventBeginPlay
  (CallFunction|MovePlatform))

(event Collision|EventActorBeginOverlap
  (params (OtherActor :type Actor%20Object%20Reference)))

(event EventTick
  (params (DeltaSeconds :type Float%20%28single-precision%29)))

(fn ConstructionScript)