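; BP_door is a trigger-driven sliding door that moves a cube between two marker positions.
; When a BP_ThirdPersonCharacter begins overlapping the box, the custom MovePlatform event runs a FlipFlop that alternates between playing the timeline from start and reversing it from end.
; The timeline's alpha lerps the cube's world location between StartPos and EndPos without sweep, so each entry toggles the direction of travel.
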(event OnComponentBeginOverlap(Box)
  (params (OverlappedComponent :type Primitive%20Component%20Object%20Reference) (OtherActor :type Actor%20Object%20Reference) (OtherComp :type Primitive%20Component%20Object%20Reference) (OtherBodyIndex :type Integer) (bFromSweep :type Boolean) (SweepResult :type Hit%20Result%20Structure%20%28by%20ref%29))
  (Utilities|Casting|CastToBP_ThirdPersonCharacter OtherActor)
  (CallFunction|MovePlatform))

(event Custom|MovePlatform
  (Utilities|FlowControl|FlipFlop
    (:A
      (bind _alpha (Timeline|Timeline PlayFromStart)
        (:Update
          (Transformation|SetWorldLocation (Variables|Default|GetCube) (Math|Vector|Lerp(Vector) (Transformation|GetWorldLocation (Variables|Default|GetstartPos)) (Transformation|GetWorldLocation (Variables|Default|GetendPos)) _alpha) false false))))
    (:B
      (Timeline|Timeline ReverseFromEnd))))

(event EventTick
  (params (DeltaSeconds :type Float%20%28single-precision%29)))

(fn ConstructionScript)