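; Basic enemy that chases the player once spotted and ends the game on contact.
; Tick halts movement until PawnSensing sees a pawn and sets IsSeeingPlayer, which is never cleared afterward.
; Each sighting triggers an AI MoveTo toward the player, playing a counter-attack animation on arrival.
; Independently of that animation, a Box overlap with the player character shows the lose screen, pauses the game and destroys the player.
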(event OnSeePawn(PawnSensing)
  (params (Pawn :type Pawn%20Object%20Reference))
  (Variables|Default|SetIsSeeingPlayer true)
  (CallFunction|FollowPlayer))

(event OnComponentBeginOverlap(Box)
  (params (OverlappedComponent :type Primitive%20Component%20Object%20Reference) (OtherActor :type Actor%20Object%20Reference) (OtherComp :type Primitive%20Component%20Object%20Reference) (OtherBodyIndex :type Integer) (bFromSweep :type Boolean) (SweepResult :type Hit%20Result%20Structure%20%28by%20ref%29))
  (bind _asbp_third_person_character (Utilities|Casting|CastToBP_ThirdPersonCharacter OtherActor))
  (bind _returnvalue (UserInterface|CreateWidget "/Game/Blueprints/LoseScreen.LoseScreen_C"))
  (UserInterface|Viewport|AddtoViewport _returnvalue 0)
  (Game|SetGamePaused true)
  (Actor|DestroyActor _asbp_third_person_character))

(event Custom|FollowPlayer
  (Variables|Default|SetcanAttack? true)
  (if (Variables|Default|GetIsSeeingPlayer)
    (AI|AIMoveTo self "0, 0, 0" (Game|GetPlayerCharacter 0) 0.0 false
      (:OnSuccess
        (if (Variables|Default|GetcanAttack?)
          (Variables|Default|SetcanAttack? false)
          (Components|Animation|PlayAnimation (Variables|Character|GetMesh) "/Game/FreeAnimationLibrary/Animations/Counter-Finisher/anim_Counter_Attack_01.anim_Counter_Attack_01" false)
          (Utilities|FlowControl|Delay 0.2)
          (Variables|Default|SetcanAttack? true))))
    (else
      (Variables|Default|SetIsSeeingPlayer false))))

(event EventBeginPlay)

(event Collision|EventActorBeginOverlap
  (params (OtherActor :type Actor%20Object%20Reference)))

(event EventTick
  (params (DeltaSeconds :type Float%20%28single-precision%29))
  (if (not (Variables|Default|GetIsSeeingPlayer))
    (Components|Movement|StopMovementImmediately (Variables|Character|GetCharacterMovement))))

(fn ConstructionScript)